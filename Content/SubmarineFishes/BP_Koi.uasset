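; BP_Koi is a koi fish Blueprint with a one-time popup triggered by its Sphere component.
; When anything begins overlapping the Sphere, it pauses the game, switches to UI-only input with the mouse cursor shown, and adds a WBP_Koi widget to the viewport.
; It then destroys the Sphere so the popup cannot fire again; unpausing and restoring input are not handled here.
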(event `self.Sphere.OnComponentBeginOverlap`
  (params (OverlappedComponent :type "PrimitiveComponent Object Reference") (OtherActor :type "Actor Object Reference") (OtherComp :type "PrimitiveComponent Object Reference") (OtherBodyIndex :type Integer) (bFromSweep :type Boolean) (SweepResult :type "HitResult Structure (by ref)"))
  (bind _returnvalue (`GameplayStatics.GetPlayerController` 0))
  (`GameplayStatics.SetGamePaused` true)
  (`WidgetBlueprintLibrary.SetInputMode_UIOnlyEx` _returnvalue null)
  (set `PlayerController.bShowMouseCursor` true _returnvalue)
  (bind _returnvalue_2 (`|CreateWidget` "/Game/UI/WBP_Koi.WBP_Koi_C" _returnvalue))
  (`UserWidget.AddToViewport` _returnvalue_2 0)
  (`ActorComponent.K2_DestroyComponent` (`self.Sphere`)))

(fn `UserConstructionScript`
  (`parent.UserConstructionScript`))